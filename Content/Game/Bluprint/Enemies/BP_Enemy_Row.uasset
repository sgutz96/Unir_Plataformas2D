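; BP_Enemy_Row is an enemy Blueprint that repeatedly fires bullets from three fire points.
; On Tick, a Sequence checks a separate CanFire flag for each point and spawns a BP_EnemyBullet at that point's world transform.
; Each branch clears its flag, then restores it after a Delay using the shared DelayFire interval, forming a simple cooldown per fire point.
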(event `self.ReceiveTick`
  (params (DeltaSeconds :type "Float (single-precision)"))
  (`|ExecutionSequence`
    (:`then_0`
      (if (`self.CanFire`)
        (set `self.CanFire` false)
        (`|SpawnActorFromClass` "/Game/Game/Bluprint/Enemies/BP_EnemyBullet.BP_EnemyBullet_C" (`SceneComponent.K2_GetComponentToWorld` (`self.FirePoint`)) "Undefined" "MultiplyWithRoot" null null)
        (`KismetSystemLibrary.Delay` (`self.DelayFire`))
        (set `self.CanFire` true)))
    (:`then_1`
      (if (`self.CanFire1`)
        (set `self.CanFire1` false)
        (`|SpawnActorFromClass` "/Game/Game/Bluprint/Enemies/BP_EnemyBullet.BP_EnemyBullet_C" (`SceneComponent.K2_GetComponentToWorld` (`self.FirePoint1`)) "Undefined" "MultiplyWithRoot" null null)
        (`KismetSystemLibrary.Delay` (`self.DelayFire`))
        (set `self.CanFire1` true)))
    (:`then_2`
      (if (`self.CanFire2`)
        (set `self.CanFire2` false)
        (`|SpawnActorFromClass` "/Game/Game/Bluprint/Enemies/BP_EnemyBullet.BP_EnemyBullet_C" (`SceneComponent.K2_GetComponentToWorld` (`self.FirePoint2`)) "Undefined" "MultiplyWithRoot" null null)
        (`KismetSystemLibrary.Delay` (`self.DelayFire`))
        (set `self.CanFire2` true)))))

(fn `UserConstructionScript`)