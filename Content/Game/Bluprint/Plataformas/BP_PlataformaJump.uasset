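; BP_PlataformaJump is a jump pad platform that launches the player character with a boosted jump.
; A hit on the Estatic component waits briefly, saves the character's JumpZVelocity, multiplies it by JumpForce and calls Jump.
; After another short delay it restores the saved velocity.
; Leaving the Box overlap also restores that saved value.
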(event `self.estatic.OnComponentHit`
  (params (HitComponent :type "PrimitiveComponent Object Reference") (OtherActor :type "Actor Object Reference") (OtherComp :type "PrimitiveComponent Object Reference") (NormalImpulse :type "Vector Structure") (Hit :type "HitResult Structure (by ref)"))
  (bind _asbp_plataform_person_character_1 (cast `/Game/Game/Bluprint/Character/BP_plataformPersonCharacter1` OtherActor))
  (`KismetSystemLibrary.Delay` 0.2)
  (bind _charactermovement (`Character.CharacterMovement` _asbp_plataform_person_character_1))
  (bind _jumpzvelocity (`CharacterMovementComponent.JumpZVelocity` _charactermovement))
  (set `self.jumpBase` _jumpzvelocity)
  (set `CharacterMovementComponent.JumpZVelocity` (* _jumpzvelocity (`self.JumpForce`)) _charactermovement)
  (`Character.Jump` _asbp_plataform_person_character_1)
  (`KismetSystemLibrary.Delay` 0.2)
  (set `CharacterMovementComponent.JumpZVelocity` (`self.jumpBase`) _charactermovement))

(event `self.Box.OnComponentEndOverlap`
  (params (OverlappedComponent :type "PrimitiveComponent Object Reference") (OtherActor :type "Actor Object Reference") (OtherComp :type "PrimitiveComponent Object Reference") (OtherBodyIndex :type Integer))
  (bind _asbp_plataform_person_character_1 (cast `/Game/Game/Bluprint/Character/BP_plataformPersonCharacter1` OtherActor))
  (set `CharacterMovementComponent.JumpZVelocity` (`self.jumpBase`) (`Character.CharacterMovement` _asbp_plataform_person_character_1)))

(fn `UserConstructionScript`)