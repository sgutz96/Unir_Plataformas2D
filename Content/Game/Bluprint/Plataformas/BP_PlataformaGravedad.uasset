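; BP_PlataformaGravedad is a platform that drops under physics after being hit, then returns.
; On a hit, the Estatic component's world location is saved to Pos, and physics simulation starts after a Duracion delay.
; Five seconds later simulation stops and MoveComponentTo sends the component back to Pos.
; The saved world position is passed as a relative-location target.
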(event `self.estatic.OnComponentHit`
  (params (HitComponent :type "PrimitiveComponent Object Reference") (OtherActor :type "Actor Object Reference") (OtherComp :type "PrimitiveComponent Object Reference") (NormalImpulse :type "Vector Structure") (Hit :type "HitResult Structure (by ref)"))
  (bind _estatic (`self.estatic`))
  (set `self.pos` (`SceneComponent.K2_GetComponentLocation` (`self.estatic`)))
  (`KismetSystemLibrary.Delay` (`self.Duracion`))
  (`PrimitiveComponent.SetSimulatePhysics` _estatic true)
  (`KismetSystemLibrary.Delay` 5.0)
  (`PrimitiveComponent.SetSimulatePhysics` _estatic false)
  (`KismetSystemLibrary.MoveComponentTo` _estatic (`self.pos`)))

(fn `UserConstructionScript`)