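; Example NPC that lets the player trigger dialogue while inside its box trigger.
; Overlap toggles the key prompt, interactable flag and input; E or DialogueManager runs the dialogue logic.
; It filters Dialogues table rows by the GameInstance's EventStatus, then fills a WBP_Dialogue widget from random matches using Spanish text.
; Portrait, line and continuation flag each use a separate Random call, so they can come from different rows.
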(event `self.ReceiveBeginPlay`)

(event `self.Box.OnComponentBeginOverlap`
  (params (OverlappedComponent :type "PrimitiveComponent Object Reference") (OtherActor :type "Actor Object Reference") (OtherComp :type "PrimitiveComponent Object Reference") (OtherBodyIndex :type Integer) (bFromSweep :type Boolean) (SweepResult :type "HitResult Structure (by ref)"))
  ; Habilitar Dialogo
  (`SceneComponent.SetVisibility` (`self.FB_KeyPress`) true false)
  (set `self.Interactuable` true)
  (`self.EnableInput` (`GameplayStatics.GetPlayerController` 0)))

(event `self.Box.OnComponentEndOverlap`
  (params (OverlappedComponent :type "PrimitiveComponent Object Reference") (OtherActor :type "Actor Object Reference") (OtherComp :type "PrimitiveComponent Object Reference") (OtherBodyIndex :type Integer))
  ; Deshabilitar Dialogo
  (`SceneComponent.SetVisibility` (`self.FB_KeyPress`) false false)
  (set `self.Interactuable` false)
  (`self.DisableInput` (`GameplayStatics.GetPlayerController` 0)))

(event `Key|E`
  (params (Key :type "Key Structure"))
  (bind _dialogues (`self.Dialogues`))
  (bind _dialogueselector (`self.DialogueSelector`))
  (bind (_id _portrait _status _connecttonext _esp) (break `/Game/Game/DialogueSystem/ST_ExampleDialogs` (`KismetArrayLibrary.Array_Random` _dialogueselector)))
  ; Gestion de dialogo a usar
  (:`Pressed`
    (if (`self.Interactuable`) :!label _label
      (`KismetArrayLibrary.Array_Clear` (`self.DialogueSelector`))
      (bind _asgi_save_data (cast `/Game/Game/Instance/GI_SaveData` (`GameplayStatics.GetGameInstance`)))
      (bind _outrownames (`DataTableFunctionLibrary.GetDataTableRowNames` _dialogues))
      (for _array_element _outrownames
        (bind _returnvalue (`|GetDataTableRow` _dialogues _array_element)
          (:`then`
            (bind (_id_2 _portrait_2 _status_2 _connecttonext_2 _esp_2 _eng) (break `/Game/Game/DialogueSystem/ST_ExampleDialogs` _returnvalue))
            (if (`KismetStringLibrary.EqualEqual_StrStr` (`KismetStringLibrary.Conv_IntToString` (`/Game/Game/Instance/GI_SaveData.EventStatus` _asgi_save_data)) (`KismetStringLibrary.Conv_IntToString` _status_2))
              (`KismetArrayLibrary.Array_AddUnique` _dialogueselector (make `/Game/Game/DialogueSystem/ST_ExampleDialogs` _id_2 _portrait_2 _status_2 _connecttonext_2 _esp_2 _eng))))))
      (bind _returnvalue_2 (`|CreateWidget` "/Game/Game/Ui/WBP_Dialogue.WBP_Dialogue_C" (`GameplayStatics.GetPlayerController` 0)))
      (set `/Game/Game/Ui/WBP_Dialogue.Image` _portrait _returnvalue_2)
      (set `/Game/Game/Ui/WBP_Dialogue.DialogueLine` (`KismetTextLibrary.Conv_StringToText` (`KismetTextLibrary.Conv_TextToString` _esp)) _returnvalue_2)
      (set `/Game/Game/Ui/WBP_Dialogue.HasNext` _connecttonext _returnvalue_2)
      (`/Game/Game/Ui/WBP_Dialogue.PlayLine` _returnvalue_2)
      (`UserWidget.AddToViewport` _returnvalue_2 0)
      (`WidgetBlueprintLibrary.SetInputMode_GameAndUIEx` (`GameplayStatics.GetPlayerController` 0) _returnvalue_2))))

(event `DialogueManager`
  ; Gestion de dialogo a usar
  (goto _label))

(fn `UserConstructionScript`)